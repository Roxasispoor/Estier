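; Capture-zone actor that tracks which flying_char pawns stand inside it and how many belong to each team.
; Begin overlap adds the character to PeopleInside and increments its team's entry in the TotalByteam map, creating it if absent.
; End overlap removes the character and decrements that count, dropping the entry at the last one.
; Counts print on screen for debugging; SetWinningTeam is an empty stub, so no winner is decided yet.
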(event `self.ReceiveActorBeginOverlap`
  (params (OtherActor :type "Actor Object Reference"))
  (bind _totalbyteam (`self.TotalByteam`))
  (bind _asflying_char (cast `/Game/blueprint/flying_char` OtherActor))
  (`KismetArrayLibrary.Array_AddUnique` (`self.People inside`) _asflying_char)
  (bind _team (`/Game/blueprint/flying_char.Team` _asflying_char))
  (bind (_value _returnvalue) (`BlueprintMapLibrary.Map_Find` _totalbyteam _team))
  (if _returnvalue
    (`BlueprintMapLibrary.Map_Add` _totalbyteam _team (+ _value 1))
    (`KismetSystemLibrary.PrintString` (`KismetStringLibrary.Conv_IntToString` _value) true true (struct :`G` 0.66 :`B` 1.0 :`A` 1.0) 2000000.0)
    (else
      (`BlueprintMapLibrary.Map_Add` _totalbyteam _team 1)
      (`KismetSystemLibrary.PrintString` (`KismetStringLibrary.Conv_IntToString` _value) true true (struct :`G` 0.66 :`B` 1.0 :`A` 1.0) 2000000.0))))

(event `self.ReceiveActorEndOverlap`
  (params (OtherActor :type "Actor Object Reference"))
  (bind _totalbyteam (`self.TotalByteam`))
  (bind _asflying_char (cast `/Game/blueprint/flying_char` OtherActor))
  (`KismetArrayLibrary.Array_RemoveItem` (`self.People inside`) _asflying_char)
  (bind _team (`/Game/blueprint/flying_char.Team` _asflying_char))
  (bind _value (`BlueprintMapLibrary.Map_Find` _totalbyteam _team))
  (if (> _value 1)
    (`BlueprintMapLibrary.Map_Add` _totalbyteam _team (- _value 1))
    (`KismetSystemLibrary.PrintString` (`KismetStringLibrary.Conv_IntToString` _value) true true (struct :`G` 0.66 :`B` 1.0 :`A` 1.0) 2000000.0)
    (else
      (`BlueprintMapLibrary.Map_Remove` _totalbyteam _team))))

(fn `SetWinningTeam`)

(fn `UserConstructionScript`)