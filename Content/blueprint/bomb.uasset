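; Bomb actor Blueprint that explodes on a timer started at BeginPlay.
; After the TimeToFuse delay it activates the Explosion component, fires a RadialForce impulse and applies radial damage around its root, passing its Instigator as the damage causer.
; It prints whether damage was applied; overlap and Tick events are unused, and nothing here destroys the actor afterwards.
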(event `self.ReceiveBeginPlay`
  (`KismetSystemLibrary.Delay` (`self.Time to fuse`))
  (`ActorComponent.Activate` (`self.explosion`) false)
  (`RadialForceComponent.FireImpulse` (`self.RadialForce`))
  (bind _returnvalue (`GameplayStatics.ApplyRadialDamage` :`BaseDamage` 30.0 :`Origin` (`SceneComponent.K2_GetComponentLocation` (`self.DefaultSceneRoot`)) :`DamageRadius` 1000.0 :`DamageCauser` (`self.GetInstigator`)))
  (`KismetSystemLibrary.PrintString` (`KismetStringLibrary.Conv_BoolToString` _returnvalue)))

(fn `UserConstructionScript`)