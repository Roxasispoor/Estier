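; Timed bomb weapon Actor that explodes after a configurable fuse delay, dealing radial damage.
; On BeginPlay it waits for the fuse, activates the explosion effect, fires a RadialForce impulse and applies full, falloff-free damage around its location, passing its instigator as damage causer.
; It then disables collision and hides its sphere components, lingering briefly before destroying itself.
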(event `self.ReceiveBeginPlay`
  (`KismetSystemLibrary.Delay` (`self.Time to fuse`))
  (`ActorComponent.Activate` (`self.explosion`) false)
  (`RadialForceComponent.FireImpulse` (`self.RadialForce`))
  (`PrimitiveComponent.SetCollisionEnabled` (`self.Sphere1`) "NoCollision")
  (`GameplayStatics.ApplyRadialDamage` :`BaseDamage` (`self.Damages`) :`Origin` (`self.K2_GetActorLocation`) :`DamageRadius` 1000.0 :`DamageCauser` (`self.GetInstigator`) :`bDoFullDamage` true)
  (`SceneComponent.SetHiddenInGame` (`self.Sphere_0`) true false)
  (`KismetSystemLibrary.Delay` 1.0)
  (`self.K2_DestroyActor`))

(fn `UserConstructionScript`)