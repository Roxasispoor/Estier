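; MaxHeal is a pickup actor that sets a flying_char's Life to 100.
; Its ApplyEffect event casts the passed object to flying_char, overwrites Life rather than adding to it, then destroys the pickup.
; It has no active overlap or tick logic of its own, so the effect depends on ApplyEffect being called.
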(event `self.Apply Effect`
  (params (NewParam :type "Actor Object Reference"))
  (bind _asflying_char (cast `/Game/blueprint/flying_char` NewParam))
  (set `/Game/blueprint/flying_char.Life` 100.0 _asflying_char)
  (`self.K2_DestroyActor`))

(fn `UserConstructionScript`
  (`parent.UserConstructionScript`))