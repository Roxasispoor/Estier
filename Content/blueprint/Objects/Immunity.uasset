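; Immunity is an effect actor that makes a flying_char invulnerable when applied.
; ApplyEffect casts the passed object to flying_char and turns off its CanBeDamaged flag.
; After a five-second delay it sets CanBeDamaged to true on itself rather than on the character, then destroys itself, so the character's flag is not restored here.
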(event `self.Apply Effect`
  (params (NewParam :type "Actor Object Reference"))
  (bind _asflying_char (cast `/Game/blueprint/flying_char` NewParam))
  (set `Actor.bCanBeDamaged` false _asflying_char)
  (`KismetSystemLibrary.Delay` 5.0)
  (set `self.bCanBeDamaged` true)
  (`self.K2_DestroyActor`))

(fn `UserConstructionScript`
  (`parent.UserConstructionScript`))