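; Game mode that manages multiplayer teams, sorting joining players into teams and supporting team switches.
; BeginPlay spawns TeamInfos actors into a Teams array, and PostLogin adds each new controller to one round-robin, using a player counter modulo TeamNumber.
; ChangeTeam locates the current team through FindPlayerTeam, moves the controller, then updates the controlled flying_char's Team reference, printing debug messages along the way.
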(event `self.ReceiveBeginPlay`
  (for _ (range (+ (`self.TeamNumber`) 1))
    (bind _returnvalue (`|SpawnActorFromClass` "/Game/blueprint/team/TeamInfos.TeamInfos_C" (`KismetMathLibrary.MakeTransform` (0.0 0.0 0.0)) "Undefined" "OverrideRootScale" null null))
    (`KismetArrayLibrary.Array_AddUnique` (`self.Teams`) _returnvalue)))

(event `self.K2_PostLogin`
  (params (NewPlayer :type "PlayerController Object Reference"))
  (`KismetArrayLibrary.Array_AddUnique` (`/Game/blueprint/team/TeamInfos.PlayersControllers` (`|GetArrayItem` (`self.Teams`) (mod (`self.PlayerNumber`) (`self.TeamNumber`)))) NewPlayer)
  (`/Engine/EditorBlueprintResources/StandardMacros.IncrementInt` (`self.PlayerNumber`)))

(fn `Change team`
  (params (`Player Controller` :type "PlayerController Object Reference") (`New Team Number` :type Integer))
  (bind _output (`|GetArrayItem` (`self.Teams`) `New Team Number`))
  (if (< `New Team Number` (`self.TeamNumber`))
    (`KismetSystemLibrary.PrintString` "imma try")
    (bind _teamtrouvee (`self.Find Player Team` `Player Controller`))
    (`KismetArrayLibrary.Array_RemoveItem` (`/Game/blueprint/team/TeamInfos.PlayersControllers` _teamtrouvee) `Player Controller`)
    (`KismetArrayLibrary.Array_AddUnique` (`/Game/blueprint/team/TeamInfos.PlayersControllers` _output) `Player Controller`)
    (bind _asflying_char (cast `/Game/blueprint/flying_char` (`Controller.K2_GetPawn` `Player Controller`))
      (:`then`
        (bind _output_get (set `/Game/blueprint/flying_char.Team` _output _asflying_char))
        (`KismetSystemLibrary.PrintString` (`KismetSystemLibrary.GetDisplayName` _output_get) true true (struct :`G` 0.66 :`B` 1.0 :`A` 1.0) 20.0))
      (:`CastFailed`
        (`KismetSystemLibrary.PrintString` "Cast failed somehow")))
    (else
      (`KismetSystemLibrary.PrintString` "mauvais numéro de team au changement"))))

(fn `Find Player Team`
  (params (`Controller to find` :type "Controller Object Reference (by ref)"))
  (returns (TeamTrouvee :type "/Game/blueprint/team/TeamInfos Object Reference"))
  (for _array_element (`self.Teams`)
    (if (!= (`KismetArrayLibrary.Array_Find` (`/Game/blueprint/team/TeamInfos.PlayersControllers` _array_element) `Controller to find`) -1)
      (return _array_element))))

(fn `UserConstructionScript`)