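; Test actor Blueprint for a UDP messaging component that talks to a local server about rooms.
; On BeginPlay it opens a UDP sender to localhost, sends two room creation commands, then requests a list after a short delay.
; Received data and decomposed room events (name and IPs) are printed on screen for debugging.
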(event `self.BPEvent_RoomDecompReceived`
  (params (nom :type String) (ips :type Integer) (playersMax :type "Integer (by ref)") (place :type "Integer (by ref)"))
  (`KismetSystemLibrary.PrintString` nom true true (struct :`R` 0.516667 :`G` 0.177946 :`B` 0.286893 :`A` 1.0) 2000.0)
  (`KismetSystemLibrary.PrintString` (`KismetStringLibrary.Conv_IntToString` ips) true true (struct :`G` 0.66 :`B` 1.0 :`A` 1.0) 2000.0))

(event `self.BPEvent_DataReceived`
  (params (receivedData :type String))
  (`KismetSystemLibrary.PrintString` receivedData true true (struct :`R` 0.989205 :`G` 1.0 :`B` 0.842533 :`A` 1.0) 2000.0))

(event `self.ReceiveBeginPlay`
  (`self.StartUDPSender` "socked" "127.0.0.1" 9999)
  (`self.SenderSendString` "create10patatausore")
  (`self.SenderSendString` "create10flausaurusRex")
  (`KismetSystemLibrary.Delay` 1.0)
  (`self.SenderSendString` "list"))

(fn `UserConstructionScript`)