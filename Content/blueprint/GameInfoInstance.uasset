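; GameInfoInstance, apparently a Game Instance, handles displaying the main, host and server menus for a game with lobby setup.
; Main and host menu widgets are created for player controller 0 on first use, cached, then re-added to the viewport.
; The server menu is created fresh on every call.
; LaunchLobby only stores the player count; its LAN and server name inputs are unused and no session is created.
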(event `ShowMainMenu`
  ;[1 1 1] Main Menu display
  (`/Engine/EditorBlueprintResources/StandardMacros.IsValid` (`self.MainMenuWB`)
    (:`Is Valid`
      _)
    (:`Is Not Valid`
      (bind _returnvalue (`|CreateWidget` "/Game/UI/MenuStuff/MainMenu.MainMenu_C" (`GameplayStatics.GetPlayerController` 0)))
      (set `self.MainMenuWB` _returnvalue)))
  (`UserWidget.AddToViewport` (`self.MainMenuWB`) 0))

(event `ShowHostMenu`
  ;[1 1 1] Host Menu Display
  (`/Engine/EditorBlueprintResources/StandardMacros.IsValid` (`self.HostMenuWB`)
    (:`Is Valid`
      _)
    (:`Is Not Valid`
      (bind _returnvalue (`|CreateWidget` "/Game/UI/MenuStuff/HostMenu.HostMenu_C" (`GameplayStatics.GetPlayerController` 0)))
      (set `self.HostMenuWB` _returnvalue)))
  (`UserWidget.AddToViewport` (`self.HostMenuWB`) 0))

(event `LaunchLobby`
  (params (NumberOfPlayer :type Integer) (`Lan?` :type Boolean) (ServerName :type String))
  (set `self.NewVar_0` NumberOfPlayer))

(event `ShowServerMenu`
  ;[1 1 1] Server Menu display - each time
  (bind _returnvalue (`|CreateWidget` "/Game/UI/MenuStuff/ServerMenu.ServerMenu_C" (`GameplayStatics.GetPlayerController` 0)))
  (`UserWidget.AddToViewport` _returnvalue 0))